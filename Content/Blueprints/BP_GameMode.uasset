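; Game mode that owns the main HUD widget, tracks the current score and keeps a persistent best score.
; BeginPlay creates WBP_Main and loads the BEST_SCORE save slot, or creates a new BP_SaveGame if the load fails.
; AddScore adds points, updates the widget, and immediately writes the save whenever the best score is beaten.
; ShowGameOver reveals the widget's GameOver element.
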(event EventBeginPlay
  ;[0.15 0.15 0.15 0.5] Main UI 만들어서 화면에 붙이자.
  (bind _returnvalue (UserInterface|CreateWidget "/Game/Blueprints/WBP_Main.WBP_Main_C"))
  (bind _output_get (Variables|Default|SetMainUI _returnvalue))
  (UserInterface|Viewport|AddtoViewport _output_get 0)
  ;[0.15 0.15 0.15 0.5] 1. BEST_SCORE 로 저장되어 있는 데이터가 있으면
  ; 2. SaveGame 변수에 불러온 데이터를 설정
  ; 3. 없으면 SaveGame 을 생성하자.
  (bind _returnvalue_2 (SaveGame|LoadGamefromSlot "BEST_SCORE"))
  (bind _asbp_save_game (Utilities|Casting|CastToBP_SaveGame _returnvalue_2)
    (:then
      (bind _output_get_2 (Variables|Default|SetSaveGame _asbp_save_game))
      (Variables|Default|SetBestScore (Variables|/Game/Blueprints/BP_SaveGame.BP_SaveGame_C|GetSaveBestScore _output_get_2)))
    (:CastFailed
      (bind _returnvalue_3 (SaveGame|CreateSaveGameObject "/Game/Blueprints/BP_SaveGame.BP_SaveGame_C"))
      (Variables|Default|SetSaveGame _returnvalue_3))))

(event EventTick
  (params (DeltaSeconds :type Float%20%28single-precision%29)))

(fn ConstructionScript)

(fn AddScore
  (params (Point :type Integer))
  (bind _savegame (Variables|Default|GetSaveGame))
  (Utilities|FlowControl|Sequence
    (:then_0
      ;[0.15 0.15 0.15 0.5] 현재 점수 Point 만큼 증가시키자.
      (Variables|Default|SetCurrScore (+ Point (Variables|Default|GetCurrScore))))
    (:then_1
      ;[0.15 0.15 0.15 0.5] 현재 점수를 Widget 에 적용하자
      (Default|UpdateScore (Variables|Default|GetMainUI) (Variables|Default|GetCurrScore)))
    (:then_2
      ;[0.15 0.15 0.15 0.5] 만약에 현재점수가 최고점수보다 크면 최고점수를 현재점수로 설정하자.
      (if (> (Variables|Default|GetCurrScore) (Variables|Default|GetBestScore))
        (bind _output_get (Variables|Default|SetBestScore (Variables|Default|GetCurrScore)))
        (Variables|/Game/Blueprints/BP_SaveGame.BP_SaveGame_C|SetSaveBestScore _savegame _output_get)
        (SaveGame|SaveGametoSlot _savegame "BEST_SCORE")))))

(fn ShowGameOver
  (Widget|SetVisibility (Variables|/Game/Blueprints/WBP_Main.WBP_Main_C|GetGameOver (Variables|Default|GetMainUI)) "Visible"))