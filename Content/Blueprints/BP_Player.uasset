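; BP_Player is the player actor, which moves in the Y-Z plane and fires bullets.
; BeginPlay adds the IMC_PlayerInput Enhanced Input mapping context.
; Tick polls the horizontal and vertical actions, normalizes the direction and offsets location by MoveSpeed and delta time, without sweep.
; The fire action spawns BP_Bullet at the FirePosition component's world transform when it starts.
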(event Input|EnhancedActionEvents|EnhancedInputActionIA_Horizontal
  (params (ActionValue :type Float%20%28double-precision%29) (ElapsedSeconds :type Float%20%28double-precision%29) (TriggeredSeconds :type Float%20%28double-precision%29) (InputAction :type Input%20Action%20Object%20Reference :default "/Game/Inputs/IA_Horizontal.IA_Horizontal")))

(event Input|EnhancedActionEvents|EnhancedInputActionIA_Fire
  (params (ActionValue :type Boolean) (ElapsedSeconds :type Float%20%28double-precision%29) (TriggeredSeconds :type Float%20%28double-precision%29) (InputAction :type Input%20Action%20Object%20Reference :default "/Game/Inputs/IA_Fire.IA_Fire"))
  (:Started
    (Game|SpawnActorfromClass "/Game/Blueprints/BP_Bullet.BP_Bullet_C" (Transformation|GetWorldTransform (Variables|Default|GetFirePosition)) "Undefined" "MultiplyWithRoot" 0 0)))

(event EventBeginPlay
  ;[0.1236 0.04906 0.15 0.5] Input Mapping Context 초기 설정
  (Input|AddMappingContext (PlayerController|LocalPlayerSubsystems|GetEnhancedInputLocalPlayerSubsystem (Game|GetPlayerController 0)) "/Game/Inputs/IMC_PlayerInput.IMC_PlayerInput" 0 "(bIgnoreAllPressedKeysUntilRelease=True,bForceImmediately=False,bNotifyUserSettings=False)"))

(event EventTick
  (params (DeltaSeconds :type Float%20%28single-precision%29))
  (Transformation|SetActorLocation (+ (* DeltaSeconds (* (Math|Vector|Normalize (Math|Vector|MakeVector 0.0 (Input|EnhancedActionValues|GetIA_Horizontal) (Input|EnhancedActionValues|GetIA_Vertical))) (Variables|Default|GetMoveSpeed))) (Transformation|GetActorLocation)) false false))

(event Collision|EventActorBeginOverlap
  (params (OtherActor :type Actor%20Object%20Reference)))

(fn ConstructionScript)