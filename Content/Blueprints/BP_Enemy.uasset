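; BP_Enemy is an enemy actor that flies in a straight line and explodes on overlap.
; On BeginPlay, a Percent-in-ten roll aims it at the player's current position and rotates it to match, otherwise it heads down.
; Tick moves it along that fixed direction.
; Overlaps, filtered by display name, skip "Destroy" actors, trigger game over for "Player", and otherwise destroy both actors with effects and score through BP_GameMode, player hits included.
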(event EventBeginPlay
  (Rendering|SetVisibility (Variables|Default|GetStaticMesh) true false)
  ;[0.15 0.15 0.15 0.5] Percent  확률로 플레어를 향하는 방향으로 설정 or 아래 방향으로 설정
  (if (< (Math|Random|RandomIntegerinRange 0 9) (Variables|Default|GetPercent))
    ;[0.15 0.15 0.15 0.5] 레벨에 있는 Player 찾아서 변수에 설정
    (bind _returnvalue (Actor|GetActorOfClass "/Game/Blueprints/BP_Player.BP_Player_C"))
    (bind _output_get (Variables|Default|SetTarget _returnvalue))
    (Utilities|IsValid _output_get
      (:Is%20Valid
        ;[0.15 0.15 0.15 0.5] Player 를 향하는 방향을 구하자 (Player위치 - Enemy위치)
        (bind _output_get_2 (Variables|Default|SetDirection (Math|Vector|Normalize (- (Transformation|GetActorLocation (Variables|Default|GetTarget)) (Transformation|GetActorLocation)))))
        ;[0.15 0.15 0.15 0.5] 액터의 앞방향 = 현재 앞방향, 액터의 윗방향 = -이동방향 으로 변경하려할 때 각도 구하는 법
        (Transformation|SetActorRotation (Math|Rotator|MakeRotfromXZ (Transformation|GetActorForwardVector) (* _output_get_2 -1.0))))
      (:Is%20Not%20Valid
        (Variables|Default|SetDirection "0.000000,0.000000,-1.000000" :!label _label)))
    (else
      (goto _label))))

(event Collision|EventActorBeginOverlap
  (params (OtherActor :type Actor%20Object%20Reference))
  (bind _returnvalue (Utilities|GetDisplayName OtherActor))
  ;[0.15 0.15 0.15 0.5] 1. 누군와 감지충돌하면
  ; 2. 충돌한 액터가 Bullet 이면 파괴하고
  ; 3. 파괴 효과 실행
  ; 4. 나도 파괴하자.
  (if (not (Utilities|String|Contains _returnvalue "Destroy"))
    (if (Utilities|String|Contains _returnvalue "Player")
      (bind _asbp_game_mode (Utilities|Casting|CastToBP_GameMode (Game|GetGameMode)))
      (Default|ShowGameOver _asbp_game_mode))
    (Actor|DestroyActor OtherActor)
    (Effects|SpawnEmitteratLocation "/Game/StarterContent/Particles/P_Explosion.P_Explosion" (Transformation|GetActorLocation)) ; 파티클 시스템 실행할 때
    (Audio|PlaySound2D "/Game/StarterContent/Audio/Explosion01.Explosion01" 1.0 1.0 0.0 0 0)
    (bind _asbp_game_mode_2 (Utilities|Casting|CastToBP_GameMode (Game|GetGameMode)))
    (Default|AddScore _asbp_game_mode_2 10)
    (Actor|DestroyActor)))

(event EventTick
  (params (DeltaSeconds :type Float%20%28single-precision%29))
  (Transformation|SetActorLocation (+ (* DeltaSeconds (* (Variables|Default|GetDirection) (Variables|Default|GetMoveSpeed))) (Transformation|GetActorLocation)) false false))

(fn ConstructionScript)